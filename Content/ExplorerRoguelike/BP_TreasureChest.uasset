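; Treasure chest Blueprint whose lid opens and closes on alternate Interact events.
; A FlipFlop plays or reverses a timeline that drives the lid mesh's relative pitch.
; An opening flag ensures the particle system activates only when the timeline finishes opening, not when it finishes closing.
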(event `ERGameplayInterface.Interact`
  (params (InstigatingPawn :type "Pawn Object Reference"))
  (`/Engine/EditorBlueprintResources/StandardMacros.FlipFlop`
    (:`A`
      (set `self.Openning` true)
      (bind (_direction _pitch) (`Timeline|ChestLidOpenTimeline` :!label _label)
        (:`Update`
          (`SceneComponent.K2_SetRelativeRotation` (`self.LidMesh`) (`KismetMathLibrary.MakeRotator` 0.0 _pitch) false false))
        (:`Finished`
          (if (`self.Openning`)
            (`ActorComponent.Activate` (`self.ParticleSystem`) false)))))
    (:`B`
      (set `self.Openning` false)
      (goto _label :!via `Reverse`))))

(fn `UserConstructionScript`)